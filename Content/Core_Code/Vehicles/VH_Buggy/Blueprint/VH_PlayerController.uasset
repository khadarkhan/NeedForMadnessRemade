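; Player controller for the buggy that tracks laps, lap times and best lap in a checkpoint race.
; An overlap event flags each of seven checkpoints by matching actor display names and notifies the HUD.
; Crossing the FinishLine trigger with all flags set, in any order, counts a lap and resets them.
; Lap time derives from the game state's total time minus cumulative time, and results go to the HUD.
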(event Custom|Event%20VH%20OverlapUpdate%20%28Controller%29
  (params (Actor :type Actor%20Object%20Reference))
  ;[1 1 1] Lap Tracking setup
  (bind _ascheck_point (Utilities|Casting|CastToCheck_point Actor)
    (:then
      (bind _asvh_hud (Utilities|Casting|CastToVH_HUD (HUD|GetHUD)))
      (Default|EventDisplayCheckpoint(HUD) _asvh_hud)
      (if (Utilities|Enum|Equal(Enum) (Utilities|GetDisplayName _ascheck_point) "Check_point")
        (Variables|Default|SetPointA true)
        (elif (Utilities|Enum|Equal(Enum) (Utilities|GetDisplayName _ascheck_point) "Check_point2")
          (Variables|Default|SetPointB true)
          (elif (Utilities|Enum|Equal(Enum) (Utilities|GetDisplayName _ascheck_point) "Check_point3")
            (Variables|Default|SetPointC true)
            (elif (Utilities|Enum|Equal(Enum) (Utilities|GetDisplayName _ascheck_point) "Check_point4")
              (Variables|Default|SetPointD true)
              (elif (Utilities|Enum|Equal(Enum) (Utilities|GetDisplayName _ascheck_point) "Check_point5")
                (Variables|Default|SetPointE true)
                (elif (Utilities|Enum|Equal(Enum) (Utilities|GetDisplayName _ascheck_point) "Check_point6")
                  (Variables|Default|SetPointF true)
                  (elif (Utilities|Enum|Equal(Enum) (Utilities|GetDisplayName _ascheck_point) "Check_point7")
                    (Variables|Default|SetPointG true)))))))))
    (:CastFailed
      (bind _astrigger_volume (Utilities|Casting|CastToTriggerVolume Actor))
      (if (Utilities|Enum|Equal(Enum) (Utilities|GetDisplayName _astrigger_volume) "FinishLine")
        (if (Variables|Default|GetPointA)
          (if (Variables|Default|GetPointB)
            (if (Variables|Default|GetPointC)
              (if (Variables|Default|GetPointD)
                (if (Variables|Default|GetPointE)
                  (if (Variables|Default|GetPointF)
                    (if (Variables|Default|GetPointG)
                      ;[1 1 1] Complete Another Lap
                      (Variables|Default|SetLapsTotal (+ (Variables|Default|GetLapsTotal) 1))
                      (Variables|Default|SetPointA false)
                      (Variables|Default|SetPointB false)
                      (Variables|Default|SetPointC false)
                      (Variables|Default|SetPointD false)
                      (Variables|Default|SetPointE false)
                      (Variables|Default|SetPointF false)
                      (Variables|Default|SetPointG false)
                      (bind _asvehicle_game_state (Utilities|Casting|CastToVehicleGameState (Game|GetGameState)))
                      (bind _returnvalue (Class|VehicleGameState|GetTotalTime _asvehicle_game_state))
                      (Variables|Default|SetLapTime (- _returnvalue (Variables|Default|GetCumulativeLapTime)))
                      (Utilities|Array|Add (Variables|Default|GetLapTimes) (- _returnvalue (Variables|Default|GetCumulativeLapTime)))
                      (if (== (Variables|Default|GetBestLapTime) 0.0)
                        (Variables|Default|SetBestLapTime (Variables|Default|GetLapTime) :!label _label)
                        (else
                          (Math|Float|CompareFloat (Variables|Default|GetLapTime) (Variables|Default|GetBestLapTime)
                            (:>
                              _)
                            (:==
                              _)
                            (:<
                              (goto _label)))))
                      (Variables|Default|SetCumulativeLapTime (+ (Variables|Default|GetLapTime) (Variables|Default|GetCumulativeLapTime)))
                      (bind _asvh_hud_2 (Utilities|Casting|CastToVH_HUD (HUD|GetHUD)))
                      (Default|EventonLapCompleted(HUD) _asvh_hud_2 (Variables|Default|GetLapsTotal) (Variables|Default|GetBestLapTime) (Variables|Default|GetCumulativeLapTime)))))))))))))

(fn ConstructionScript)